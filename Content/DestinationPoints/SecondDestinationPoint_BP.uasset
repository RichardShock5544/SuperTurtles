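; SecondDestinationPoint_BP is a destination trigger that makes the SecondTurtle_BP actor vanish in a puff of fog.
; Any overlap on its Box looks up the first SecondTurtle_BP in the level, without checking which actor entered.
; A chain of Delays then activates the turtle's Fog, hides its Mesh with a 2D Poof sound, deactivates the fog and destroys the turtle.
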(event `self.Box.OnComponentBeginOverlap`
  (params (OverlappedComponent :type "PrimitiveComponent Object Reference") (OtherActor :type "Actor Object Reference") (OtherComp :type "PrimitiveComponent Object Reference") (OtherBodyIndex :type Integer) (bFromSweep :type Boolean) (SweepResult :type "HitResult Structure (by ref)"))
  (bind _outactors (`GameplayStatics.GetAllActorsOfClass` "/Game/Turtles/SecondTurtle_BP.SecondTurtle_BP_C"))
  (bind _output (`|GetArrayItem` _outactors))
  (`ActorComponent.Activate` (`/Game/Turtles/TurtleParent_BP.Fog` _output) false)
  (`KismetSystemLibrary.Delay` 0.7)
  (`SceneComponent.SetVisibility` (`Character.Mesh` _output) false false)
  (`GameplayStatics.PlaySound2D` "/Game/SFX/poof.poof" 1.0 1.0 0.0 null null)
  (`KismetSystemLibrary.Delay` 1.5)
  (`ActorComponent.Deactivate` (`/Game/Turtles/TurtleParent_BP.Fog` _output))
  (`KismetSystemLibrary.Delay` 1.0)
  (`self.K2_DestroyActor` _output))

(fn `UserConstructionScript`
  (`parent.UserConstructionScript`))