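; 2ndPit_BP is a pit Blueprint whose only active logic is a short flash effect on its point light.
; The LightOn event steps the light through sharply varying intensities with brief delays, then sets it to zero.
; Nothing in this graph calls LightOn, and the BeginPlay, overlap and Tick events are disabled stubs.
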(event `LightOn`
  (`LightComponent.SetIntensity` (`self.PointLight`) 50000.0)
  (`KismetSystemLibrary.Delay` 0.1)
  (`LightComponent.SetIntensity` (`self.PointLight`) 500000.0)
  (`KismetSystemLibrary.Delay` 0.1)
  (`LightComponent.SetIntensity` (`self.PointLight`) 100000.0)
  (`KismetSystemLibrary.Delay` 0.1)
  (`LightComponent.SetIntensity` (`self.PointLight`) 250000.0)
  (`KismetSystemLibrary.Delay` 0.1)
  (`LightComponent.SetIntensity` (`self.PointLight`) 0.0))

(fn `UserConstructionScript`
  (`parent.UserConstructionScript`))