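; SecondTurtle_BP is a turtle pawn that heads toward a finish point in a repeating move-and-pause rhythm, starting on BeginPlay.
; GoForward issues an AI move to the Finish component of the first SecondDestinationPoint_BP found in the level.
; Without waiting for arrival, it delays, calls StopMovementImmediately on CharacterMovement, delays briefly, then calls itself again.
; An unconnected variant of this movement chain never runs.
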(event `self.ReceiveBeginPlay`
  (`parent.ReceiveBeginPlay`)
  (`self.GoForward`))

(event `GoForward`
  (bind _outactors (`GameplayStatics.GetAllActorsOfClass` "/Game/DestinationPoints/SecondDestinationPoint_BP.SecondDestinationPoint_BP_C"))
  (`|AIMoveTo` self (`SceneComponent.K2_GetComponentLocation` (`/Game/DestinationPoints/ParentDestinationPoint_BP.finish` (`|GetArrayItem` _outactors))) null
    (:`then`
      (`KismetSystemLibrary.Delay` 1.0)
      (`MovementComponent.StopMovementImmediately` (`self.CharacterMovement`))
      (`KismetSystemLibrary.Delay` 0.5)
      (`self.GoForward`))))

(fn `UserConstructionScript`
  (`parent.UserConstructionScript`))